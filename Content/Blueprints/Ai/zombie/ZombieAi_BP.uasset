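; Zombie AI character that randomizes its walk speed on spawn and handles health, hit reactions, attacks and death.
; AnyDamage reduces health while alive, then triggers either Death or a hit montage with a debug damage print.
; Hit, attack and death montages play through a shared PlayAnimM helper that calls RandomMontage.
; Death switches the mesh to physics ragdoll shortly before its montage ends, then destroys the actor after a delay.
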(event Custom|ZombieAttack
  (CallFunction|PlayAnimM (Variables|Default|GetAttackMontage) 0 1 1.0 "None"))

(event Custom|Death
  (Variables|Default|SetDead true)
  (bind _returnvalue (CallFunction|PlayAnimM (Variables|Default|GetDeathMontage) 0 1 1.0 "None"))
  (Utilities|FlowControl|Delay (- _returnvalue 0.5))
  (Collision|SetCollisionProfileName (Variables|Character|GetMesh) (Utilities|Name|MakeLiteralName "Ragdoll") true :!class /Script/Engine.PrimitiveComponent)
  (Physics|SetSimulatePhysics (Variables|Character|GetMesh) true)
  (Utilities|FlowControl|Delay 5.0)
  (Actor|DestroyActor))

(event Custom|Damage
  (params (Damage :type Float%20%28single-precision%29))
  (CallFunction|PlayAnimM (Variables|Default|GetMontage) 0 1 1.0 "None")
  (Development|PrintString (Utilities|String|ToString(Float) Damage)))

(event EventBeginPlay
  (Variables|/Script/Engine.CharacterMovementComponent|SetMaxWalkSpeed (Variables|Character|GetCharacterMovement) (Math|Random|RandomFloatinRange 7e+01 2e+02)))

(event Collision|EventActorBeginOverlap
  (params (OtherActor :type Actor%20Object%20Reference)))

(event EventTick
  (params (DeltaSeconds :type Float%20%28single-precision%29)))

(event Game|Damage|EventAnyDamage
  (params (Damage :type Float%20%28single-precision%29) (DamageType :type Damage%20Type%20Object%20Reference) (InstigatedBy :type Controller%20Object%20Reference) (DamageCauser :type Actor%20Object%20Reference))
  (if (not (Variables|Default|GetDead))
    (Variables|Default|SetHealth (- (Variables|Default|GetHealth) Damage))
    (if (<= (Variables|Default|GetHealth) 0.0)
      (CallFunction|Death)
      (else
        (CallFunction|Damage Damage)))))

(fn ConstructionScript)

(fn PlayAnimM
  (params (Array :type Array%20of%20Anim%20Montage%20Object%20References) (Min :type Integer) (Max :type Integer) (InPlayRate :type Float%20%28single-precision%29) (StartSectionName :type Name))
  (bind _returnvalue (Animation|PlayAnimMontage (Utilities|RandomMontage Array Min Max) InPlayRate StartSectionName))
  (return _returnvalue))