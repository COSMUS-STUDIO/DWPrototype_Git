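; AttackingState is an animation notify state that marks the active attack window in BP_Aki's animations.
; On begin it sets the character's IsAttacking flag, and on each tick it calls the character's Trace function.
; On end it clears the flag and calls ClearDamaged.
; All three events act only when the mesh owner casts to BP_Aki.
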(fn ReceivedNotifyBegin
  (params (MeshComp :type Skeletal%20Mesh%20Component%20Object%20Reference) (Animation :type Anim%20Sequence%20Base%20Object%20Reference) (TotalDuration :type Float%20%28single-precision%29))
  (bind _asbp_aki (Utilities|Casting|CastToBP_Aki (Components|GetOwner MeshComp)))
  (Variables|/Game/Blueprints/BP_Aki.BP_Aki_C|SetisAttacking _asbp_aki true)
  (return false))

(fn ReceivedNotifyEnd
  (params (MeshComp :type Skeletal%20Mesh%20Component%20Object%20Reference) (Animation :type Anim%20Sequence%20Base%20Object%20Reference))
  (bind _asbp_aki (Utilities|Casting|CastToBP_Aki (Components|GetOwner MeshComp)))
  (Variables|/Game/Blueprints/BP_Aki.BP_Aki_C|SetisAttacking _asbp_aki false)
  (Default|ClearDamaged _asbp_aki)
  (return false))

(fn ReceivedNotifyTick
  (params (MeshComp :type Skeletal%20Mesh%20Component%20Object%20Reference) (Animation :type Anim%20Sequence%20Base%20Object%20Reference) (FrameDeltaTime :type Float%20%28single-precision%29))
  (bind _asbp_aki (Utilities|Casting|CastToBP_Aki (Components|GetOwner MeshComp)))
  (Default|Trace _asbp_aki)
  (return false))